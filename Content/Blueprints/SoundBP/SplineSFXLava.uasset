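; Lava ambience actor that slides a lava sound along a spline so it plays from the point nearest the player.
; On BeginPlay it caches the FirstPersonCharacter and starts MoveAudio, which moves the audio component to the closest spline location, raised slightly in Z.
; MoveAudio re-calls itself after a short Delay, giving a polling loop without using Tick.
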(event Custom|Move%20Audio
  (bind _char_ref (Variables|Default|GetChar%20REF))
  (bind _spline (Variables|Default|GetSpline))
  (bind _returnvalue (Transformation|GetActorLocation _char_ref))
  (bind _returnvalue_2 (Spline|FindLocationClosesttoWorldLocation _spline _returnvalue "World"))
  (bind _result (Math|Float|IncrementFloat (.z _returnvalue_2))
    (:%20%20
      (Transformation|SetWorldLocation (Variables|Default|GetSFX_Environment_Lava_Cue) (Math|Vector|MakeVector (.x _returnvalue_2) (.y _returnvalue_2) _result) false false)
      (Utilities|FlowControl|Delay 0.05)
      (CallFunction|MoveAudio))))

(event EventBeginPlay
  (bind _asfirst_person_character (Utilities|Casting|CastToFirstPersonCharacter (Game|GetPlayerCharacter 0)))
  (Variables|Default|SetChar%20REF _asfirst_person_character)
  (CallFunction|MoveAudio))

(fn ConstructionScript)